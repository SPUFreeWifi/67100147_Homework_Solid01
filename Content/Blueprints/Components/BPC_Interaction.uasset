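; Player character component that finds nearby interactable actors, shows an interaction prompt and triggers their interaction.
; Each tick a sphere trace around the owner updates the found list, which takes new actors only when empty.
; The "closest" is actually the first passing a view-angle check, whose 200-degree limit never excludes by angle.
; A screen-space widget shows that target's text at its location, and Interact messages the same pick, then delists it.
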(event `self.ReceiveBeginPlay`
  (bind _interactwidgetcomp (`self.InteractWidgetComp`))
  (bind _asbp_player_character (cast `/Game/Blueprints/ThirdPerson/Blueprints/BP_Player_Character` (`self.GetOwner`)))
  (bind _output_get (set `self.OwnerCharacter` _asbp_player_character))
  (bind _returnvalue (`|AddComponentByClass` _output_get "/Script/UMG.WidgetComponent" true (`KismetMathLibrary.MakeTransform` (0.0 0.0 0.0))))
  (set `self.InteractWidgetComp` _returnvalue)
  (`|ExecutionSequence`
    (:`then_0`
      (`WidgetComponent.SetDrawSize` _interactwidgetcomp (400.0 50.0))
      (`WidgetComponent.SetWidgetSpace` _interactwidgetcomp "Screen"))
    (:`then_1`
      (bind _returnvalue_2 (`|CreateWidget` "/Game/Blueprints/Widgets/WBP_Interact.WBP_Interact_C"))
      (bind _output_get_2 (set `self.InteractWidget` _returnvalue_2))
      (`Widget.SetVisibility` _output_get_2 "Collapsed"))
    (:`then_2`
      (`WidgetComponent.SetWidget` (`self.InteractWidgetComp`) (`self.InteractWidget`)))))

(event `self.ReceiveTick`
  (params (DeltaSeconds :type "Float (single-precision)"))
  (bind _closest_interactable (`self.Closest Interactable`))
  (`/Engine/EditorBlueprintResources/StandardMacros.IsValid` (`self.OwnerCharacter`)
    (:`Is Valid`
      (`|ExecutionSequence`
        (:`then_0`
          (`self.findInteractables`))
        (:`then_1`
          (bind _returnclosestinteractable (`self.FindClosestInteractable`))
          (`/Engine/EditorBlueprintResources/StandardMacros.IsValid` _returnclosestinteractable
            (:`Is Valid`
              (if (!= _returnclosestinteractable (`self.Closest Interactable`))
                (set `self.Closest Interactable` _returnclosestinteractable)
                (`|ExecutionSequence`
                  (:`then_0`
                    (`Widget.SetVisibility` (`self.InteractWidget`) "Visible"))
                  (:`then_1`
                    (bind _returnvector (message `/Game/Blueprints/Interface/BPI_Interactable.GetInteractTextLocation` _closest_interactable))
                    (`SceneComponent.K2_SetWorldLocation` (`self.InteractWidgetComp`) _returnvector false false)
                    (bind _returntext (message `/Game/Blueprints/Interface/BPI_Interactable.GetInteractText` _closest_interactable))
                    (`/Game/Blueprints/Widgets/WBP_Interact.SetInteractText` (`self.InteractWidget`) _returntext)))))
            (:`Is Not Valid`
              (set `self.Closest Interactable` null)
              (`Widget.SetVisibility` (`self.InteractWidget`) "Collapsed"))))))))

(fn `FindClosestInteractable`
  (returns (ReturnClosestInteractable :type "Actor Object Reference"))
  (bind _foundinteractables (`self.FoundInteractables`))
  (if (`KismetArrayLibrary.Array_IsNotEmpty` _foundinteractables)
    (for _array_element _foundinteractables
      (if (`self.IsInteractableInViewLengh` _array_element)
        (return _array_element))))
  (return null))

(fn `findInteractables`
  (locals (TmpInteractables :type "Array of Actor Object Reference"))
  (bind _foundinteractables (`self.FoundInteractables`))
  (bind _returnvalue (`Actor.K2_GetActorLocation` (`self.GetOwner`)))
  (bind (_outhits _returnvalue_2) (`KismetSystemLibrary.SphereTraceMulti` _returnvalue _returnvalue 100.0 "TraceTypeQuery1"))
  (if _returnvalue_2
    ; Add Tmp Interactables
    (for _array_element _outhits
      (bind (_bblockinghit _binitialoverlap _time _distance _location _impactpoint _normal _impactnormal _physmat _hitactor) (`GameplayStatics.BreakHitResult` _array_element))
      (bind _returniscan (message `/Game/Blueprints/Interface/BPI_Interactable.CanInteractable` _hitactor))
      (if (and _bblockinghit _returniscan)
        (`KismetArrayLibrary.Array_Add` (`local.TmpInteractables`) _hitactor)))
    (if (`KismetArrayLibrary.Array_IsEmpty` (`self.FoundInteractables`))
      (`KismetArrayLibrary.Array_Append` (`self.FoundInteractables`) (`local.TmpInteractables`))
      (else
        (bind (_arrayindex _arrayelement) (`/Engine/EditorBlueprintResources/StandardMacros.ReverseForEachLoop` _foundinteractables)
          (:`LoopBody`
            (if (not (`KismetArrayLibrary.Array_Contains` (`local.TmpInteractables`) _arrayelement))
              (`KismetArrayLibrary.Array_RemoveItem` _foundinteractables _arrayelement))))))
    (else
      (`KismetArrayLibrary.Array_Clear` (`self.FoundInteractables`)))))

(fn `Interact`
  (locals (TempInteractable :type "Actor Object Reference"))
  (bind _foundinteractables (`self.FoundInteractables`))
  (bind _tempinteractable (`local.TempInteractable`))
  (if (`KismetArrayLibrary.Array_IsNotEmpty` _foundinteractables)
    (for _array_element _foundinteractables
      (if (`self.IsInteractableInViewLengh` _array_element)
        (set `local.TempInteractable` _array_element)
        (break)))
    (`/Engine/EditorBlueprintResources/StandardMacros.IsValid` _tempinteractable
      (:`Is Valid`
        (`|ExecutionSequence`
          (:`then_0`
            (message `/Game/Blueprints/Interface/BPI_Interactable.OnInteract` _tempinteractable (`self.OwnerCharacter`)))
          (:`then_1`
            (`KismetArrayLibrary.Array_RemoveItem` (`self.FoundInteractables`) _tempinteractable)))))))

(fn `IsInteractableInViewLengh`
  (params (Interactable :type "Actor Object Reference"))
  (returns (ReturnValue :type Boolean))
  (return (<= (`KismetMathLibrary.DegAcos` (`KismetMathLibrary.Dot_VectorVector` (`KismetMathLibrary.GetForwardVector` (`Pawn.GetControlRotation` (`self.OwnerCharacter`))) (`KismetMathLibrary.Normal` (- (`Actor.K2_GetActorLocation` Interactable) (`Actor.K2_GetActorLocation` (`self.GetOwner`)))))) 200.0)))