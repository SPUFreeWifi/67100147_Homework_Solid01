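; Base interactable actor that acts as an inventory pickup, exposing interaction checks and prompt data.
; OnInteract sets IsInteract, prints a debug message, adds InventoryItemClass to the interacter's BPC_Inventory component, then destroys the actor.
; CanInteractable returns false once interacted, while GetInteractText and GetInteractTextLocation supply a prompt built from the display name and the actor's location.
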(event `/Game/Blueprints/Interface/BPI_Interactable.OnInteract`
  (params (Interacter :type "/Game/Blueprints/ThirdPerson/Blueprints/BP_ThirdPersonCharacter Object Reference"))
  (`|ExecutionSequence`
    (:`then_0`
      (set `self.IsInteract` true))
    (:`then_1`
      (`KismetSystemLibrary.PrintText` (`|FormatText` "Interact : {Object}" (`KismetSystemLibrary.GetObjectName` self))))
    (:`then_2`
      (`/Game/Blueprints/Inventory/BPC_Inventory.AddItem` (`self.GetComponentByClass` Interacter "/Game/Blueprints/Inventory/BPC_Inventory.BPC_Inventory_C") (`self.Inventory item class`))
      (`self.K2_DestroyActor`))))

(fn `CanInteractable`
  (returns (ReturnIsCan :type Boolean))
  (return (not (`self.IsInteract`))))

(fn `GetInteractText`
  (returns (ReturnText :type Text))
  (return (`|FormatText` "Interact at : {Object}" (`KismetSystemLibrary.GetDisplayName` self))))

(fn `GetInteractTextLocation`
  (returns (ReturnVector :type "Vector Structure"))
  (return (`self.K2_GetActorLocation`)))

(fn `UserConstructionScript`)