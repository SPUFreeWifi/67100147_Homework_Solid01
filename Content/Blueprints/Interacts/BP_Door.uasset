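; BP_Door is an interactable door that shows an "Open Door" prompt at its text point and swings open when used.
; On interact, it sets a motion warping target at its interact point and plays a door-opening montage on the interacting character.
; When the montage completes or is interrupted, it clears the interact flag and plays a timeline that rotates the door pivot open.
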(event `/Game/Blueprints/Interface/BPI_Interactable.OnInteract`
  (params (Interacter :type "/Game/Blueprints/ThirdPerson/Blueprints/BP_ThirdPersonCharacter Object Reference"))
  (bind _interact_point (`self.Interact Point`))
  (`parent.OnInteract` Interacter)
  (`MotionWarpingComponent.AddOrUpdateWarpTargetFromLocationAndRotation` (`/Game/Blueprints/ThirdPerson/Blueprints/BP_ThirdPersonCharacter.MotionWarping` Interacter) "InteractTarget2" (`SceneComponent.K2_GetComponentLocation` _interact_point) (`SceneComponent.K2_GetComponentRotation` _interact_point))
  (`|PlayMontage` (`Character.Mesh` Interacter) "/Game/Assets/Animations/AM_OpenDoor_R_Montage.AM_OpenDoor_R_Montage"
    (:`OnCompleted`
      _)
    (:`OnInterrupted`
      _))
  (set `self.IsInteract` false)
  (bind (_direction _alpha) (`Timeline|DoorTimeLine`)
    (:`Update`
      (`SceneComponent.K2_SetRelativeRotation` (`self.DoorPivot`) (`KismetMathLibrary.RLerp` (struct) (struct :`Yaw` -90.0) _alpha) false false))))

(fn `GetInteractText`
  (returns (ReturnText :type Text))
  (return "Open Door"))

(fn `GetInteractTextLocation`
  (returns (ReturnVector :type "Vector Structure"))
  (return (`SceneComponent.K2_GetComponentLocation` (`self.InteractTextPoint`))))

(fn `UserConstructionScript`
  (`parent.UserConstructionScript`))